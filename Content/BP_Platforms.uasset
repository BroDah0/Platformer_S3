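; BP_Platforms is a colored platform actor that starts solid or non-collidable according to its IsBlue flag.
; The construction script applies the blue "on" material when IsBlue is set, otherwise the editor brush material with collision disabled.
; A SwitchPlatform event is meant for toggling but is unfinished: it checks collision state, while both collision-setting nodes remain disconnected.
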(event EventBeginPlay)

(event Collision|EventActorBeginOverlap
  (params (OtherActor :type Actor%20Object%20Reference)))

(event EventTick
  (params (DeltaSeconds :type Float%20%28single-precision%29)))

(event EventSwitchPlatform
  (if (Class|PrimitiveComponent|IsCollisionEnabled (Variables|Default|GetPlatform))
    _))

(fn ConstructionScript
  (bind _platform (Variables|Default|GetPlatform))
  (if (Variables|Default|GetIsBlue)
    (Rendering|Material|SetMaterial _platform 0 "/Engine/VREditor/UI/BluePlatformOn.BluePlatformOn")
    (else
      (Rendering|Material|SetMaterial _platform 0 "/Engine/EngineMaterials/EditorBrushMaterial.EditorBrushMaterial")
      (Collision|SetCollisionEnabled (Variables|Default|GetPlatform) "NoCollision"))))